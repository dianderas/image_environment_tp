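; BP_PuertaDormitorio is a bedroom door that moves automatically when the player enters or leaves its trigger Box.
; Overlap by player pawn 0 plays the Movimiento timeline, and ending the overlap reverses it.
; The timeline's Apertura track drives the Cube's relative Z location, keeping X and Y unchanged, so the door slides vertically.
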(event OnComponentBeginOverlap(Box)
  (params (OverlappedComponent :type Primitive%20Component%20Object%20Reference) (OtherActor :type Actor%20Object%20Reference) (OtherComp :type Primitive%20Component%20Object%20Reference) (OtherBodyIndex :type Integer) (bFromSweep :type Boolean) (SweepResult :type Hit%20Result%20Structure%20%28by%20ref%29))
  (bind _cube (Variables|Default|GetCube))
  (bind _relativelocation (Variables|/Script/Engine.SceneComponent|GetRelativeLocation _cube))
  ;[0.05913 0.004533 0.1094] Ingreso del jugador
  (if (== OtherActor (Game|Player|GetPlayerPawn 0))
    ;[0.3961 0.07181 1] Puerta
    (bind _apertura (Timeline|Movimiento Play)
      (:Update
        (Transformation|SetRelativeLocation _cube (Math|Vector|MakeVector (.x _relativelocation) (.y _relativelocation) _apertura) false false)))))

(event OnComponentEndOverlap(Box)
  (params (OverlappedComponent :type Primitive%20Component%20Object%20Reference) (OtherActor :type Actor%20Object%20Reference) (OtherComp :type Primitive%20Component%20Object%20Reference) (OtherBodyIndex :type Integer))
  (bind _cube (Variables|Default|GetCube))
  (bind _relativelocation (Variables|/Script/Engine.SceneComponent|GetRelativeLocation _cube))
  ;[0.05913 0.004533 0.1094] Ingreso del jugador
  (if (== OtherActor (Game|Player|GetPlayerPawn 0))
    ;[0.3961 0.07181 1] Puerta
    (bind _apertura (Timeline|Movimiento Reverse)
      (:Update
        (Transformation|SetRelativeLocation _cube (Math|Vector|MakeVector (.x _relativelocation) (.y _relativelocation) _apertura) false false)))))

(fn ConstructionScript)