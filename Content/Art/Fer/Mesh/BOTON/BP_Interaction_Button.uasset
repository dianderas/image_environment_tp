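; Interactable button that toggles a level sequence forward and in reverse when the player presses it.
; A Box overlap with the player character shows or removes a widget prompt and sets the proximity flag that gates the IA_PressButton input.
; An open-state flag picks the playback direction on LevelSequenceActor.
; BeginPlay enables input, creates the prompt and creates a player for the BEGIN_PLAY sequence without starting it.
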(event OnComponentBeginOverlap(Box)
  (params (OverlappedComponent :type Primitive%20Component%20Object%20Reference) (OtherActor :type Actor%20Object%20Reference) (OtherComp :type Primitive%20Component%20Object%20Reference) (OtherBodyIndex :type Integer) (bFromSweep :type Boolean) (SweepResult :type Hit%20Result%20Structure%20%28by%20ref%29))
  (if (== OtherActor (Game|GetPlayerCharacter 0))
    (UserInterface|Viewport|AddtoViewport (Variables|Default|GetInteractPrompt) 0)
    (Variables|Default|SetisNerby true)))

(event OnComponentEndOverlap(Box)
  (params (OverlappedComponent :type Primitive%20Component%20Object%20Reference) (OtherActor :type Actor%20Object%20Reference) (OtherComp :type Primitive%20Component%20Object%20Reference) (OtherBodyIndex :type Integer))
  (if (== (Game|GetPlayerCharacter 0) OtherActor)
    (Widget|RemovefromParent (Variables|Default|GetInteractPrompt))
    (Variables|Default|SetisNerby false)))

(event Input|EnhancedActionEvents|EnhancedInputActionIA_PressButton
  (params (ActionValue :type Boolean) (ElapsedSeconds :type Float%20%28double-precision%29) (TriggeredSeconds :type Float%20%28double-precision%29) (InputAction :type Input%20Action%20Object%20Reference :default "/Game/FirstPerson/Input/Actions/IA_PressButton.IA_PressButton"))
  (bind _level_sequence_actor (Variables|Default|GetLevel%20Sequence%20Actor))
  (bind _sequenceplayer (Variables|/Script/LevelSequence.LevelSequenceActor|GetSequencePlayer _level_sequence_actor))
  (:Started
    (if (Variables|Default|GetisNerby)
      (if (Variables|Default|GetisOpen)
        (Class|MovieSceneSequencePlayer|PlayReverse _sequenceplayer)
        (Variables|Default|SetisOpen false)
        (else
          (Sequencer|Player|Play _sequenceplayer :!class /Script/MovieScene.MovieSceneSequencePlayer)
          (Variables|Default|SetisOpen true))))))

(event EventBeginPlay
  (Input|EnableInput (Game|GetPlayerController 0))
  (bind _returnvalue (UserInterface|CreateWidget "/Game/Art/Fer/Mesh/BOTON/WB_Interation_Button.WB_Interation_Button_C"))
  (Variables|Default|SetInteractPrompt _returnvalue)
  (Sequencer|Player|CreateLevelSequencePlayer "/Game/Art/ANIMACION/BEGIN_PLAY.BEGIN_PLAY"))

(fn ConstructionScript)