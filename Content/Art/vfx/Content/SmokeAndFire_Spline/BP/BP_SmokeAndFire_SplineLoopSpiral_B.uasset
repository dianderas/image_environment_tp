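; Looping spiral spline fire-and-smoke effect actor that exposes a Niagara Fluids system's settings as Blueprint variables.
; The Construction Script pushes them into FXFireAndSmokeSplineLoop: spline motion, volume, sources, smoke, fire, forces, boundaries and secondary particles; the event graph is inactive.
; A Movie Render Queue toggle also pushes resolution and pressure-iteration overrides.
; LifetimeMax is written to "Lifetime Min", overwriting LifetimeMin and leaving the maximum unset.
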(event EventBeginPlay)

(event Collision|EventActorBeginOverlap
  (params (OtherActor :type Actor%20Object%20Reference)))

(event EventTick
  (params (DeltaSeconds :type Float%20%28single-precision%29)))

(fn ConstructionScript
  (bind _fx_fireandsmoke_splineloop (Variables|Default|GetFX_FireAndSmoke_SplineLoop))
  (bind _fx_fireandsmoke_splineloop_2 (Variables|Default|GetFX_FireAndSmoke_SplineLoop))
  (bind _fx_fireandsmoke_splineloop_3 (Variables|Default|GetFX_FireAndSmoke_SplineLoop))
  (bind _fx_fireandsmoke_splineloop_4 (Variables|Default|GetFX_FireAndSmoke_SplineLoop))
  (bind _fx_fireandsmoke_splineloop_5 (Variables|Default|GetFX_FireAndSmoke_SplineLoop))
  (bind _fx_fireandsmoke_splineloop_6 (Variables|Default|GetFX_FireAndSmoke_SplineLoop))
  (bind _fx_fireandsmoke_splineloop_7 (Variables|Default|GetFX_FireAndSmoke_SplineLoop))
  (bind _fx_fireandsmoke_splineloop_8 (Variables|Default|GetFX_FireAndSmoke_SplineLoop))
  (bind _fx_fireandsmoke_splineloop_9 (Variables|Default|GetFX_FireAndSmoke_SplineLoop))
  (bind _fx_fireandsmoke_splineloop_10 (Variables|Default|GetFX_FireAndSmoke_SplineLoop))
  (bind _fx_fireandsmoke_splineloop_11 (Variables|Default|GetFX_FireAndSmoke_SplineLoop))
  (bind _fx_fireandsmoke_splineloop_12 (Variables|Default|GetFX_FireAndSmoke_SplineLoop))
  ;[1 1 1] Spline
  (Niagara|SetNiagaraVariable(Float) _fx_fireandsmoke_splineloop_12 "Speed" (Variables|Spline|GetSpeed))
  (Niagara|SetNiagaraVariable(Float) _fx_fireandsmoke_splineloop_12 "Loop" (Variables|Spline|GetLoop))
  ;[1 1 1] Niagara Fluids - Volume
  (Class|NiagaraComponent|SetVariableInt _fx_fireandsmoke_splineloop_2 "Resolution Max Axis" (Variables|NiagaraFluids-Volume|GetResolution%20Max%20Axis))
  (Class|NiagaraComponent|SetVariableBool _fx_fireandsmoke_splineloop_2 "Draw Bounds" (Variables|NiagaraFluids-Volume|GetDraw%20Bounds))
  (Niagara|SetNiagaraVariable(Vector3) _fx_fireandsmoke_splineloop_2 "Volume Size" (Variables|NiagaraFluids-Volume|GetVolume%20Size))
  (Class|NiagaraComponent|SetNiagaraVariableInt _fx_fireandsmoke_splineloop_2 "Pressure Solve Iterations" (Variables|NiagaraFluids-Volume|GetPressure%20Solve%20Iterations))
  ;[1 1 1] Niagara Fluids Movie Render Queue
  (if (Variables|MovieRenderQueue|GetRender%20with%20MovieRenderQueue?)
    (Class|NiagaraComponent|SetNiagaraVariableInt _fx_fireandsmoke_splineloop_3 "Override Resolution Max Axis" (Variables|MovieRenderQueue|GetOverride%20Resolution%20Max%20Axis))
    (Class|NiagaraComponent|SetNiagaraVariableInt _fx_fireandsmoke_splineloop_3 "Override Pressure Solve Iterations" (Variables|MovieRenderQueue|GetOverride%20Pressure%20Solve%20Iterations)))
  ;[1 1 1] Niagara Fluids - Particles
  (Niagara|SetNiagaraVariable(Float) _fx_fireandsmoke_splineloop_4 "SpawnRate " (Variables|NiagaraFluids-Particles|GetSpawnRate))
  (Niagara|SetNiagaraVariable(Float) _fx_fireandsmoke_splineloop_4 "Lifetime Min" (Variables|NiagaraFluids-Particles|GetLifetime%20Min))
  (Niagara|SetNiagaraVariable(Float) _fx_fireandsmoke_splineloop_4 "Lifetime Min" (Variables|NiagaraFluids-Particles|GetLifetime%20Max))
  (Niagara|SetNiagaraVariable(Float) _fx_fireandsmoke_splineloop_4 "Uniform Sprite Size Min" (Variables|NiagaraFluids-Particles|GetUniform%20Sprite%20Size%20Min))
  (Niagara|SetNiagaraVariable(Float) _fx_fireandsmoke_splineloop_4 "Uniform Sprite Size Max" (Variables|NiagaraFluids-Particles|GetUniform%20Sprite%20Size%20Max))
  (Niagara|SetNiagaraVariable(Float) _fx_fireandsmoke_splineloop_4 "Noise Strength" (Variables|NiagaraFluids-Particles|GetNoise%20Strength))
  (Niagara|SetNiagaraVariable(Float) _fx_fireandsmoke_splineloop_4 "Noise Frequency" (Variables|NiagaraFluids-Particles|GetNoise%20Frequency))
  (Niagara|SetNiagaraVariable(Float) _fx_fireandsmoke_splineloop_4 "Vortex Force Amount" (Variables|NiagaraFluids-Particles|GetVortex%20Force%20Amount))
  (Niagara|SetNiagaraVariable(Vector3) _fx_fireandsmoke_splineloop_4 "Vortex Axis" (Variables|NiagaraFluids-Particles|GetVortex%20Axis))
  (Niagara|SetNiagaraVariable(Float) _fx_fireandsmoke_splineloop_4 "Drag" (Variables|NiagaraFluids-Particles|GetDrag))
  ;[1 1 1] Niagara Fluids - Source Parameters
  (Niagara|SetNiagaraVariable(Float) _fx_fireandsmoke_splineloop_5 "Minimum_Radius" (Variables|NiagaraFluids-SourceParameters|GetMinimum_Radius))
  (Niagara|SetNiagaraVariable(Float) _fx_fireandsmoke_splineloop_5 "Maximum_Radius" (Variables|NiagaraFluids-SourceParameters|GetMaximum_Radius))
  (Niagara|SetNiagaraVariable(Float) _fx_fireandsmoke_splineloop_5 "Divergence" (Variables|NiagaraFluids-SourceParameters|GetDivergence))
  (Niagara|SetNiagaraVariable(Float) _fx_fireandsmoke_splineloop_5 "Velocity Scale" (Variables|NiagaraFluids-SourceParameters|GetVelocity%20Scale))
  (Niagara|SetNiagaraVariable(Vector3) _fx_fireandsmoke_splineloop_5 "Gravity" (Variables|NiagaraFluids-SourceParameters|GetGravity))
  ;[1 1 1] Niagara Fluids - Smoke
  (Niagara|SetNiagaraVariable(LinearColor) _fx_fireandsmoke_splineloop_6 "Smoke Color" (Variables|NiagaraFluids-Smoke|GetSmoke%20Color))
  (Niagara|SetNiagaraVariable(Float) _fx_fireandsmoke_splineloop_6 "Smoke Density" (Variables|NiagaraFluids-Smoke|GetSmoke%20Density))
  (Niagara|SetNiagaraVariable(Float) _fx_fireandsmoke_splineloop_6 "Smoke Buoyancy" (Variables|NiagaraFluids-Smoke|GetSmoke%20Buoyancy))
  (Niagara|SetNiagaraVariable(Float) _fx_fireandsmoke_splineloop_6 "Smoke Dissipation Rate " (Variables|NiagaraFluids-Smoke|GetSmoke%20Dissipation%20Rate%20))
  (Niagara|SetNiagaraVariable(Float) _fx_fireandsmoke_splineloop_6 "Smoke Albedo" (Variables|NiagaraFluids-Smoke|GetSmoke%20Albedo))
  (Niagara|SetNiagaraVariable(Float) _fx_fireandsmoke_splineloop_6 "Smoke Gain" (Variables|NiagaraFluids-Smoke|GetSmoke%20Gain))
  ;[1 1 1] Niagara Fluids - Fire
  (Niagara|SetNiagaraVariable(Float) _fx_fireandsmoke_splineloop_7 "Fire Temperature" (Variables|NiagaraFluids-Fire|GetFire%20Temperature))
  (Niagara|SetNiagaraVariable(Float) _fx_fireandsmoke_splineloop_7 "Fire Buoyancy" (Variables|NiagaraFluids-Fire|GetFire%20Buoyancy))
  (Niagara|SetNiagaraVariable(Float) _fx_fireandsmoke_splineloop_7 "Fire Dissipation Rate " (Variables|NiagaraFluids-Fire|GetFire%20Dissipation%20Rate%20))
  (Niagara|SetNiagaraVariable(Float) _fx_fireandsmoke_splineloop_7 "Fire Opacity Gain" (Variables|NiagaraFluids-Fire|GetFire%20Opacity%20Gain))
  (Niagara|SetNiagaraVariable(Float) _fx_fireandsmoke_splineloop_7 "Fire Color Gain" (Variables|NiagaraFluids-Fire|GetFire%20Color%20Gain))
  ;[1 1 1] Niagara Fluids - Forces
  (Niagara|SetNiagaraVariable(Float) _fx_fireandsmoke_splineloop_8 "Vorticity" (Variables|NiagaraFluids-Forces|GetVorticity))
  (Niagara|SetNiagaraVariable(Float) _fx_fireandsmoke_splineloop_8 "Initial Turbulence Frequency" (Variables|NiagaraFluids-Forces|GetInitial%20Turbulence%20Frequency))
  (Niagara|SetNiagaraVariable(Float) _fx_fireandsmoke_splineloop_8 "Initial Turbulence Gain" (Variables|NiagaraFluids-Forces|GetInitial%20Turbulence%20Gain))
  (Niagara|SetNiagaraVariable(Float) _fx_fireandsmoke_splineloop_8 "Turbulence 1 Frequency" (Variables|NiagaraFluids-Forces|GetTurbulence%201%20Frequency))
  (Niagara|SetNiagaraVariable(Float) _fx_fireandsmoke_splineloop_8 "Turbulence 1 Gain" (Variables|NiagaraFluids-Forces|GetTurbulence%201%20Gain))
  (Niagara|SetNiagaraVariable(Float) _fx_fireandsmoke_splineloop_8 "Small Scale Turbulence Block Size" (Variables|NiagaraFluids-Forces|GetSmall%20Scale%20Turbulence%20Block%20Size))
  (Niagara|SetNiagaraVariable(Float) _fx_fireandsmoke_splineloop_8 "Small Scale Turbulence Gain" (Variables|NiagaraFluids-Forces|GetSmall%20Scale%20Turbulence%20Gain))
  (Niagara|SetNiagaraVariable(Float) _fx_fireandsmoke_splineloop_8 "Wind Strength" (Variables|NiagaraFluids-Forces|GetWind%20Strength))
  (Niagara|SetNiagaraVariable(Vector3) _fx_fireandsmoke_splineloop_8 "Wind Direction" (Variables|NiagaraFluids-Forces|GetWind%20Direction))
  ;[1 1 1] Niagara Fluids - Collisions
  (Class|NiagaraComponent|SetVariableBool _fx_fireandsmoke_splineloop_9 "Open Boundary -X" (Variables|NiagaraFluids-Collisions|GetOpen%20Boundary%20-X))
  (Class|NiagaraComponent|SetVariableBool _fx_fireandsmoke_splineloop_9 "Open Boundary +X" (Variables|NiagaraFluids-Collisions|GetOpen%20Boundary%20+X))
  (Class|NiagaraComponent|SetVariableBool _fx_fireandsmoke_splineloop_9 "Open Boundary -Y" (Variables|NiagaraFluids-Collisions|GetOpen%20Boundary%20-Y))
  (Class|NiagaraComponent|SetVariableBool _fx_fireandsmoke_splineloop_9 "Open Boundary +Y" (Variables|NiagaraFluids-Collisions|GetOpen%20Boundary%20+Y))
  (Class|NiagaraComponent|SetVariableBool _fx_fireandsmoke_splineloop_9 "Open Boundary -Z" (Variables|NiagaraFluids-Collisions|GetOpen%20Boundary%20-Z))
  (Class|NiagaraComponent|SetVariableBool _fx_fireandsmoke_splineloop_9 "Open Boundary +Z" (Variables|NiagaraFluids-Collisions|GetOpen%20Boundary%20+Z))
  ;[1 1 1] Particles - Parameters
  (Niagara|SetNiagaraVariable(Float) _fx_fireandsmoke_splineloop_10 "Particles SpawnRate" (Variables|Particles-Parameters|GetParticles%20SpawnRate))
  (Niagara|SetNiagaraVariable(Float) _fx_fireandsmoke_splineloop_10 "Particles Lifetime Min" (Variables|Particles-Parameters|GetParticles%20Lifetime%20Min))
  (Niagara|SetNiagaraVariable(Float) _fx_fireandsmoke_splineloop_10 "Particles Lifetime Max" (Variables|Particles-Parameters|GetParticles%20Lifetime%20Max))
  (Niagara|SetNiagaraVariable(Float) _fx_fireandsmoke_splineloop_10 "Particles Sprite Size Min" (Variables|Particles-Parameters|GetParticles%20Sprite%20Size%20Min))
  (Niagara|SetNiagaraVariable(Float) _fx_fireandsmoke_splineloop_10 "Particles Sprite Size Max" (Variables|Particles-Parameters|GetParticles%20Sprite%20Size%20Max))
  (Niagara|SetNiagaraVariable(LinearColor) _fx_fireandsmoke_splineloop_10 "Particles ColorA" (Variables|Particles-Parameters|GetParticles%20ColorA))
  (Niagara|SetNiagaraVariable(LinearColor) _fx_fireandsmoke_splineloop_10 "Particles ColorB" (Variables|Particles-Parameters|GetParticles%20ColorB))
  ;[1 1 1] Particles - Forces
  (Niagara|SetNiagaraVariable(Float) _fx_fireandsmoke_splineloop_11 "Particles Noise Strength" (Variables|Particles-Forces|GetParticles%20Noise%20Strength))
  (Niagara|SetNiagaraVariable(Float) _fx_fireandsmoke_splineloop_11 "Particles Noise Frequency" (Variables|Particles-Forces|GetParticles%20Noise%20Frequency))
  (Niagara|SetNiagaraVariable(Float) _fx_fireandsmoke_splineloop_11 "Particles Drag" (Variables|Particles-Forces|GetParticles%20Drag))
  (Niagara|SetNiagaraVariable(Vector3) _fx_fireandsmoke_splineloop_11 "Particles Wind Speed" (Variables|Particles-Forces|GetParticles%20Wind%20Speed))
  (Niagara|SetNiagaraVariable(Float) _fx_fireandsmoke_splineloop_11 "Particles Wind Turbulence Fequency" (Variables|Particles-Forces|GetParticles%20Wind%20Turbulence%20Fequency))
  (Niagara|SetNiagaraVariable(Float) _fx_fireandsmoke_splineloop_11 "Particles Vortex Force" (Variables|Particles-Forces|GetParticles%20Vortex%20Force))
  (Niagara|SetNiagaraVariable(Vector3) _fx_fireandsmoke_splineloop_11 "Particles  Vortex Axis" (Variables|Particles-Forces|GetParticles%20%20Vortex%20Axis))
  ;[1 1 1] Particles - Collisions
  (Class|NiagaraComponent|SetVariableBool _fx_fireandsmoke_splineloop "Collision Enabled" (Variables|Particles-Collisions|GetCollision%20Enabled))
  (Niagara|SetNiagaraVariable(Float) _fx_fireandsmoke_splineloop "Particles Friction" (Variables|Particles-Collisions|GetParticles%20Friction))
  (Niagara|SetNiagaraVariable(Float) _fx_fireandsmoke_splineloop "Particles Bounce Restitution" (Variables|Particles-Collisions|GetParticles%20Bounce%20Restitution)))